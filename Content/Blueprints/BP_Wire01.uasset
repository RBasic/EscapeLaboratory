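; Construction-script wire actor that builds spline meshes along its Spline in one of several wire variants.
; SplineMeshVar picks the layout: one segment per pair of spline points, or segments at fixed Spacing with scaled tangents.
; Both layouts share one path that scales each segment and creates MI_Wire dynamic materials.
; Some variants take a second material slot, and parameters drive colour, dirt, specular, roughness and texture set.
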(fn ConstructionScript
  (|Wire))